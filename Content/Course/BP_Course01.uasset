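; BP_Course01 is a course piece that reacts when an actor overlaps its Course01 component.
; The construction script creates a dynamic instance of MT_Course, assigns it to the component and sets its BaseColor to light gray.
; Begin overlap turns the material red and plays the Shok_M_Cue sound at the overlapping actor's location, and end overlap restores the gray.
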(event OnComponentBeginOverlap(Course01)
  (params (OverlappedComponent :type Primitive%20Component%20Object%20Reference) (OtherActor :type Actor%20Object%20Reference) (OtherComp :type Primitive%20Component%20Object%20Reference) (OtherBodyIndex :type Integer) (bFromSweep :type Boolean) (SweepResult :type Hit%20Result%20Structure%20%28by%20ref%29))
  (Rendering|Material|SetVectorParameterValue (Variables|Default|GetCourse_Material) "BaseColor" "(R=1.000000,G=0.000000,B=0.000000,A=1.000000)" :!class /Script/Engine.MaterialInstanceDynamic)
  (Audio|SpawnSoundatLocation "/Game/Cue/Shok_M_Cue.Shok_M_Cue" (Transformation|GetActorLocation OtherActor) "0, 0, 0" 1.0 1.0 0.0 0 0))

(event OnComponentEndOverlap(Course01)
  (params (OverlappedComponent :type Primitive%20Component%20Object%20Reference) (OtherActor :type Actor%20Object%20Reference) (OtherComp :type Primitive%20Component%20Object%20Reference) (OtherBodyIndex :type Integer))
  (Rendering|Material|SetVectorParameterValue (Variables|Default|GetCourse_Material) "BaseColor" "(R=0.886275,G=0.886275,B=0.886275,A=1.000000)" :!class /Script/Engine.MaterialInstanceDynamic))

(fn ConstructionScript
  (bind _returnvalue (Rendering|Material|CreateDynamicMaterialInstance "/Game/Course/MT_Course.MT_Course" "" "None" :!class /Script/Engine.KismetMaterialLibrary))
  (bind _output_get (Variables|Default|SetCourse_Material _returnvalue))
  (Rendering|Material|SetMaterial (Variables|Default|GetCourse01) 0 _output_get)
  (Rendering|Material|SetVectorParameterValue _output_get "BaseColor" "(R=0.885417,G=0.885417,B=0.885417,A=1.000000)" :!class /Script/Engine.MaterialInstanceDynamic))